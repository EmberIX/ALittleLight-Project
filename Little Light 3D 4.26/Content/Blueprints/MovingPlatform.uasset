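; Light-activated moving platform that ping-pongs along a Track spline while lit and stops when no light remains.
; Box overlaps track light sources (lantern-carrying player, lit lanterns, Koopas, pillars) in LightList.
; The Lit timeline fades the Appearance material parameter, then starts or stops movement, where a FlipFlop alternates Moving timeline direction with a short pause.
; Cube overlap snaps a lantern the player is not carrying onto the platform's Arrow.
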(event `self.ReceiveTick`
  (params (DeltaSeconds :type "Float (single-precision)")))

(event `self.ReceiveBeginPlay`
  (`MeshComponent.SetScalarParameterValueOnMaterials` (`self.Root`) "Appearance" 1.0))

(event `Active`
  (bind _spline (`/Game/Blueprints/TrackRef.Spline` (`self.Track`)))
  ;[1 1 1] Activated
  (if (not (`self.isActivated`))
    (`KismetSystemLibrary.PrintString` "Activate")
    (set `self.isActivated` true)
    (`/Engine/EditorBlueprintResources/StandardMacros.FlipFlop` :!label _label
      (:`A`
        (bind (_direction _travel) (`Timeline|Moving` :!label _label_2)
          (:`Update`
            (bind _returnvalue (* _travel (`SplineComponent.GetSplineLength` (`/Game/Blueprints/TrackRef.Spline` (`self.Track`)))))
            (bind (_returnvalue_roll _returnvalue_pitch _returnvalue_yaw) (`KismetMathLibrary.BreakRotator` (`SplineComponent.GetRotationAtDistanceAlongSpline` _spline _returnvalue "World")))
            (`self.K2_SetActorLocationAndRotation` (`SplineComponent.GetLocationAtDistanceAlongSpline` _spline _returnvalue "World") (`KismetMathLibrary.MakeRotator` _returnvalue_roll 0.0 _returnvalue_yaw)))
          (:`Finished`
            (`KismetSystemLibrary.Delay` 0.5)
            (goto _label))))
      (:`B`
        (goto _label_2 :!via `Reverse`)))))

(event `DeActivate`
  ;[1 1 1] Deactivated
  (`KismetSystemLibrary.PrintString` "Deactivated")
  (`TimelineComponent.Stop` (`self.Moving`)))

(event `self.Cube.OnComponentBeginOverlap`
  (params (OverlappedComponent :type "PrimitiveComponent Object Reference") (OtherActor :type "Actor Object Reference") (OtherComp :type "PrimitiveComponent Object Reference") (OtherBodyIndex :type Integer) (bFromSweep :type Boolean) (SweepResult :type "HitResult Structure (by ref)"))
  ;[1 1 1] Lantern
  (bind _aslantern_bp (cast `/Game/Blueprints/Lantern_BP` OtherActor))
  (if (`PrimitiveComponent.IsOverlappingComponent` (`/Game/Blueprints/Lantern_BP.Capsule` _aslantern_bp) OverlappedComponent)
    (bind _asthird_person_character (cast `/Game/Blueprints/ThirdPersonCharacter` (`GameplayStatics.GetPlayerPawn` 0)))
    (if (not (`/Game/Blueprints/ThirdPersonCharacter.IsLantern` _asthird_person_character))
      (bind _output_get (set `self.As Lantern BP` _aslantern_bp))
      (`self.K2_AttachToComponent` _output_get (`self.Arrow`) "None" "SnapToTarget" "SnapToTarget" "SnapToTarget" false)
      (set `/Game/Blueprints/Lantern_BP.OnPlatform` true _output_get)
      (set `/Game/Blueprints/Lantern_BP.Platform` self _output_get))))

(event `self.Box.OnComponentBeginOverlap`
  (params (OverlappedComponent :type "PrimitiveComponent Object Reference") (OtherActor :type "Actor Object Reference") (OtherComp :type "PrimitiveComponent Object Reference") (OtherBodyIndex :type Integer) (bFromSweep :type Boolean) (SweepResult :type "HitResult Structure (by ref)"))
  ;[1 1 1] BeginOverlap
  (`|ExecutionSequence`
    (:`then_0`
      (bind _asthird_person_character (cast `/Game/Blueprints/ThirdPersonCharacter` OtherActor))
      (if (`/Game/Blueprints/ThirdPersonCharacter.IsLantern` _asthird_person_character)
        (if (not (`/Game/Blueprints/ThirdPersonCharacter.LightChanged` _asthird_person_character))
          (`KismetArrayLibrary.Array_Add` (`self.LightList`) _asthird_person_character)
          (`KismetSystemLibrary.PrintString` "In light" :!label _label_3)
          (if (not (`self.isInlight`))
            (`|ExecutionSequence` :!label _label_4
              (:`then_0`
                (if (> (`KismetArrayLibrary.Array_Length` (`self.LightList`)) 0)
                  (bind (_direction _lit) (`Timeline|Lit` :!label _label_5)
                    (:`Update`
                      (`MeshComponent.SetScalarParameterValueOnMaterials` (`self.Root`) "Appearance" (`KismetMathLibrary.Lerp` 1.0 0.0 _lit)))
                    (:`Finished`
                      (if (`|EnumEquality` _direction "Forward")
                        (set `self.isInlight` true)
                        (`self.Active`)
                        (else
                          (set `self.isInlight` false)
                          (`self.DeActivate`)
                          (set `self.isActivated` false))))))))))))
    (:`then_1`
      (bind _aslantern_bp (cast `/Game/Blueprints/Lantern_BP` OtherActor))
      (if (`/Game/Blueprints/Lantern_BP.isLight` _aslantern_bp)
        (`KismetArrayLibrary.Array_Add` (`self.LightList`) _aslantern_bp)
        (goto _label_3)))
    (:`then_2`
      (bind _askoopa_bp2 (cast `/Game/Blueprints/Koopa_BP2` OtherActor))
      (`KismetArrayLibrary.Array_Add` (`self.LightList`) _askoopa_bp2)
      (goto _label_4))
    (:`then_3`
      (bind _aspillar (cast `/Game/Blueprints/Pillar` OtherActor))
      (`KismetArrayLibrary.Array_Add` (`self.LightList`) _aspillar)
      (goto _label_4))
    (:`then_4`
      (bind _asbroken_pillar (cast `/Game/Blueprints/BrokenPillar` OtherActor))
      (if (`PrimitiveComponent.IsOverlappingComponent` (`/Game/Blueprints/BrokenPillar.Sphere1` _asbroken_pillar) OverlappedComponent)
        (if (`/Game/Blueprints/BrokenPillar.isLight` _asbroken_pillar)
          (`KismetArrayLibrary.Array_Add` (`self.LightList`) _asbroken_pillar)
          (goto _label_3))))))

(event `self.Box.OnComponentEndOverlap`
  (params (OverlappedComponent :type "PrimitiveComponent Object Reference") (OtherActor :type "Actor Object Reference") (OtherComp :type "PrimitiveComponent Object Reference") (OtherBodyIndex :type Integer))
  (if (`self.isInlight`)
    (`|ExecutionSequence`
      (:`then_0`
        (bind _asthird_person_character (cast `/Game/Blueprints/ThirdPersonCharacter` OtherActor))
        (if (`/Game/Blueprints/ThirdPersonCharacter.IsLantern` _asthird_person_character)
          (if (`/Game/Blueprints/ThirdPersonCharacter.LightChanged` _asthird_person_character)
            _
            (elif (not (`PrimitiveComponent.IsOverlappingComponent` (`/Game/Blueprints/ThirdPersonCharacter.Sphere` _asthird_person_character) OverlappedComponent))
              (`KismetArrayLibrary.Array_RemoveItem` (`self.LightList`) _asthird_person_character)
              (if (not (> (`KismetArrayLibrary.Array_Length` (`self.LightList`)) 0)) :!label _label_6
                (goto _label_5 :!via `Reverse`))))))
      (:`then_1`
        (bind _aslantern_bp (cast `/Game/Blueprints/Lantern_BP` OtherActor))
        (if (`PrimitiveComponent.IsOverlappingComponent` (`/Game/Blueprints/Lantern_BP.LanternLightCol` _aslantern_bp) OverlappedComponent)
          _
          (elif (`/Game/Blueprints/Lantern_BP.isLight` _aslantern_bp)
            (`KismetArrayLibrary.Array_RemoveItem` (`self.LightList`) _aslantern_bp)
            (goto _label_6))))
      (:`then_2`
        (bind _askoopa_bp2 (cast `/Game/Blueprints/Koopa_BP2` OtherActor))
        (if (not (`PrimitiveComponent.IsOverlappingComponent` (`/Game/Blueprints/Koopa_BP2.SightRangee` _askoopa_bp2) OverlappedComponent))
          (`KismetArrayLibrary.Array_RemoveItem` (`self.LightList`) _askoopa_bp2)
          (goto _label_6)))
      (:`then_3`
        (bind _aspillar (cast `/Game/Blueprints/Pillar` OtherActor))
        (`KismetArrayLibrary.Array_RemoveItem` (`self.LightList`) _aspillar)
        (goto _label_6))
      (:`then_4`
        (bind _asbroken_pillar (cast `/Game/Blueprints/BrokenPillar` OtherActor))
        (if (`PrimitiveComponent.IsOverlappingComponent` (`/Game/Blueprints/BrokenPillar.Sphere1` _asbroken_pillar) OverlappedComponent)
          _
          (elif (`/Game/Blueprints/BrokenPillar.isLight` _asbroken_pillar)
            (`KismetArrayLibrary.Array_RemoveItem` (`self.LightList`) _asbroken_pillar)
            (goto _label_6)))))))

(fn `UserConstructionScript`)