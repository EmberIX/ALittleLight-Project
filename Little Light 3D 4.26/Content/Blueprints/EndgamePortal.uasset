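; EndgamePortal is a portal actor that sends the player to MainScene once its Activate flag is true.
; Tick mirrors the flag onto the visibility of the Col component and its children.
; When a ThirdPersonCharacter overlaps component E while active, it adds a Fading widget to the viewport, waits briefly, then opens the level by name.
; Nothing in this graph sets Activate.
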(event `self.ReceiveTick`
  (params (DeltaSeconds :type "Float (single-precision)"))
  (bind _col (`self.col`))
  (if (`self.Activate`)
    (`SceneComponent.SetVisibility` _col true true)
    (else
      (`SceneComponent.SetVisibility` _col false true))))

(event `self.e.OnComponentBeginOverlap`
  (params (OverlappedComponent :type "PrimitiveComponent Object Reference") (OtherActor :type "Actor Object Reference") (OtherComp :type "PrimitiveComponent Object Reference") (OtherBodyIndex :type Integer) (bFromSweep :type Boolean) (SweepResult :type "HitResult Structure (by ref)"))
  (cast `/Game/Blueprints/ThirdPersonCharacter` OtherActor)
  (if (`self.Activate`)
    (bind _returnvalue (`|CreateWidget` "/Game/Widget/UI/Fading.Fading_C" (`GameplayStatics.GetPlayerController` 0)))
    (`UserWidget.AddToViewport` _returnvalue 0)
    (`KismetSystemLibrary.Delay` 1.0)
    (`GameplayStatics.OpenLevel` "MainScene")))

(fn `UserConstructionScript`)