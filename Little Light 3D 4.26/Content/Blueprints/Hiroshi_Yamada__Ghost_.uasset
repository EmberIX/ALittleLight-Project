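; Hiroshi Yamada ghost that patrols back and forth between two waypoints.
; On BeginPlay it caches the world locations of two waypoint components, then chains AI MoveTo calls to each, looping back after the second succeeds.
; It pauses briefly and prints a debug greeting at the first point.
; Failed moves are unhandled, so the patrol stops if one fails.
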(event `self.ReceiveBeginPlay`
  (set `self.WayPts01_Vec` (`SceneComponent.K2_GetComponentLocation` (`self.Waypts01`)))
  (set `self.WayPts02_Vec` (`SceneComponent.K2_GetComponentLocation` (`self.Waypts02`)))
  (`|AIMoveTo` self (`self.WayPts01_Vec`) null 0.0 :!label _label
    (:`OnSuccess`
      (`KismetSystemLibrary.Delay` 0.2)
      (`KismetSystemLibrary.PrintString` "Hello")
      (`|AIMoveTo` self (`self.WayPts02_Vec`) null 0.0
        (:`OnSuccess`
          (goto _label))))))

(fn `UserConstructionScript`)