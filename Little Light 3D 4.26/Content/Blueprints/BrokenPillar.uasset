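; Broken pillar that the player can light temporarily by grabbing while inside its trigger, provided the character's LightChanged flag is off.
; Lighting swaps the ball material, shows particles, and uses timelines to grow a collision sphere and light, then reverses them after a delay.
; Tick polls the grab, counts down the lit time, shows a floating widget via a nearby sphere trace, and yaws the UI circle toward the player.
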(event `self.ReceiveBeginPlay`
  (set `self.MaxDelayTime` 60.0)
  (`SceneComponent.SetVisibility` (`self.ParticleSystem`) false false)
  (bind _asfloaty_broken_pilar_ui (cast `/Game/Widget/UI/Floaty_BrokenPilarUI` (`WidgetComponent.GetWidget` (`self.Widget`))))
  (set `/Game/Widget/UI/Floaty_BrokenPilarUI.As Broken Pillar` self _asfloaty_broken_pilar_ui))

(event `self.ReceiveTick`
  (params (DeltaSeconds :type "Float (single-precision)"))
  (bind _returnvalue (`self.K2_GetActorLocation`))
  (bind _widget (`self.Widget`))
  (`|ExecutionSequence`
    (:`then_0`
      (if (`self.isAtPillar`)
        (bind _asthird_person_character (cast `/Game/Blueprints/ThirdPersonCharacter` (`GameplayStatics.GetPlayerCharacter` 0)))
        (if (`/Game/Blueprints/ThirdPersonCharacter.LightChanged` _asthird_person_character)
          _
          (elif (`/Game/Blueprints/ThirdPersonCharacter.Grab` _asthird_person_character)
            (`self.LightPillar`)))))
    (:`then_1`
      (bind (_outhit _returnvalue_2) (`KismetSystemLibrary.SphereTraceSingleForObjects` _returnvalue _returnvalue 90.0 (`|MakeArray` "ObjectTypeQuery3" :!type "EObjectTypeQuery Enum") true))
      (if _returnvalue_2
        (cast `/Game/Blueprints/ThirdPersonCharacter` (`.HitActor` (`GameplayStatics.BreakHitResult` _outhit)))
        (`SceneComponent.SetVisibility` _widget true false)
        (else
          (`SceneComponent.SetVisibility` _widget false false))))
    (:`then_2`
      (`SceneComponent.K2_SetRelativeRotation` (`self.UICircle`) (`KismetMathLibrary.MakeRotator` 0.0 0.0 (.yaw (`KismetMathLibrary.FindLookAtRotation` (`SceneComponent.K2_GetComponentLocation` (`self.UICircle`)) (`self.K2_GetActorLocation` (`GameplayStatics.GetPlayerPawn` 0))))) false false))
    (:`then_3`
      (if (`self.isLight`)
        (set `self.DelayTime` (- (`self.DelayTime`) DeltaSeconds))))))

(event `LightPillar`
  (set `self.isLight` true)
  (set `self.DelayTime` (`self.MaxDelayTime`))
  (`PrimitiveComponent.SetMaterial` (`self.Ball`) 0 "/Game/Meterial/LightBall.LightBall")
  (bind (_direction _lightcol _light_intensity) (`Timeline|FadeIn` :!via `PlayFromStart`)
    (:`Update`
      (`PrimitiveComponent.SetCollisionEnabled` (`self.Sphere1`) "QueryOnly")
      (`SphereComponent.SetSphereRadius` (`self.Sphere1`) _lightcol true)
      (`LightComponent.SetIntensity` (`self.PointLight`) _light_intensity)
      (`SceneComponent.SetVisibility` (`self.ParticleSystem`) true false))
    (:`Finished`
      (`KismetSystemLibrary.Delay` (`self.DelayTime`))
      (bind (_direction_2 _lightcol_2 _light_intensity_2) (`Timeline|FadeOut` :!via `ReverseFromEnd`)
        (:`Update`
          (`SphereComponent.SetSphereRadius` (`self.Sphere1`) _lightcol_2 true)
          (`LightComponent.SetIntensity` (`self.PointLight`) _light_intensity_2))
        (:`Finished`
          (set `self.isLight` false)
          (`PrimitiveComponent.SetMaterial` (`self.Ball`) 0 "/Game/StarterContent/Props/Materials/M_StatueGlass.M_StatueGlass")
          (`PrimitiveComponent.SetCollisionEnabled` (`self.Sphere1`) "NoCollision")
          (`SceneComponent.SetVisibility` (`self.ParticleSystem`) false false))))))

(event `self.PillarCol.OnComponentBeginOverlap`
  (params (OverlappedComponent :type "PrimitiveComponent Object Reference") (OtherActor :type "Actor Object Reference") (OtherComp :type "PrimitiveComponent Object Reference") (OtherBodyIndex :type Integer) (bFromSweep :type Boolean) (SweepResult :type "HitResult Structure (by ref)"))
  (bind _asthird_person_character (cast `/Game/Blueprints/ThirdPersonCharacter` OtherActor))
  (if (`PrimitiveComponent.IsOverlappingComponent` (`Character.CapsuleComponent` _asthird_person_character) OverlappedComponent)
    (set `self.isAtPillar` true)))

(event `self.PillarCol.OnComponentEndOverlap`
  (params (OverlappedComponent :type "PrimitiveComponent Object Reference") (OtherActor :type "Actor Object Reference") (OtherComp :type "PrimitiveComponent Object Reference") (OtherBodyIndex :type Integer))
  (bind _asthird_person_character (cast `/Game/Blueprints/ThirdPersonCharacter` OtherActor))
  (if (`PrimitiveComponent.IsOverlappingComponent` (`Character.CapsuleComponent` _asthird_person_character) OverlappedComponent)
    _
    (else
      _))
  (set `self.isAtPillar` false))

(fn `UserConstructionScript`)