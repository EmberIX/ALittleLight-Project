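; Interactable altar that takes the player's carried lantern to transfer life source into a tree and activate the endgame portal.
; Interact casts the attached item to Lantern_BP, destroys it, clears the character's carry state and sets Activate on itself and the EndgamePortal.
; A DialogueBox widget toggles the message and locks walking while open; later interactions only toggle it.
; Tick keeps the particle system visible once activated.
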(event `/Game/Widget/UI/Interact_I.Interact`
  (bind _player (`self.player`))
  (if (`self.Activate`)
    (`self.Dialogue`)
    (else
      (bind _asthird_person_character (cast `/Game/Blueprints/ThirdPersonCharacter` (`GameplayStatics.GetPlayerPawn` 0)))
      (bind _currentattach (`/Game/Blueprints/ThirdPersonCharacter.CurrentAttach` _asthird_person_character))
      (bind _aslantern_bp (cast `/Game/Blueprints/Lantern_BP` _currentattach))
      (set `self.player` _asthird_person_character)
      (`/Engine/EditorBlueprintResources/StandardMacros.IsValid` _aslantern_bp
        (:`Is Valid`
          (`self.K2_DestroyActor` _currentattach)
          (set `/Game/Blueprints/ThirdPersonCharacter.IsLantern` false _player)
          (set `self.Activate` true)
          (set `self.Text` "Life source has transfer in to the tree.")
          (`self.Dialogue`)
          (`/Game/Blueprints/ThirdPersonCharacter.Lantern!` _player)
          (set `/Game/Blueprints/ThirdPersonCharacter.CurrentAttach` null _player)
          (set `/Game/Blueprints/ThirdPersonCharacter.isAttach` false _player)
          (`self.Activated`))
        (:`Is Not Valid`
          (`self.Dialogue`))))))

(event `self.ReceiveTick`
  (params (DeltaSeconds :type "Float (single-precision)"))
  (if (`self.Activate`)
    (`SceneComponent.SetVisibility` (`self.ParticleSystem`) true false)))

(event `Dialogue`
  (`/Engine/EditorBlueprintResources/StandardMacros.IsValid` (`self.DialogueWidget`)
    (:`Is Valid`
      (`Widget.RemoveFromParent` (`self.DialogueWidget`))
      (set `self.DialogueWidget` null)
      (bind _asthird_person_character (cast `/Game/Blueprints/ThirdPersonCharacter` (`GameplayStatics.GetPlayerPawn` 0)))
      (set `/Game/Blueprints/ThirdPersonCharacter.CanWalk` true _asthird_person_character))
    (:`Is Not Valid`
      (bind _returnvalue (`|CreateWidget` "/Game/Widget/UI/DialogueBox.DialogueBox_C" (`GameplayStatics.GetPlayerController` 0)))
      (bind _output_get (set `self.DialogueWidget` _returnvalue))
      (`UserWidget.AddToViewport` _output_get 0)
      (set `/Game/Widget/UI/DialogueBox.DialogueText` (`self.Text`) (`self.DialogueWidget`))
      (bind _asthird_person_character_2 (cast `/Game/Blueprints/ThirdPersonCharacter` (`GameplayStatics.GetPlayerPawn` 0)))
      (set `/Game/Blueprints/ThirdPersonCharacter.CanWalk` false _asthird_person_character_2))))

(event `Activated`
  (`KismetSystemLibrary.PrintString` "activated")
  (bind _asendgame_portal (cast `/Game/Blueprints/EndgamePortal` (`self.EndGamePortal`)))
  (set `/Game/Blueprints/EndgamePortal.Activate` true _asendgame_portal))

(fn `UserConstructionScript`)