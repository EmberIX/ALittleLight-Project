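; FloatyObject is an actor that bobs up and down in place.
; Tick adds a small swept local Z offset, with a latent Delay flipping TransformUp about every second to reverse direction.
; A short random startup delay sets EndDelay, staggering the start of motion between instances.
; The yaw scaled by DeltaSeconds leaves the Z axis unchanged, so the step is fixed per frame and the actor never rotates.
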(event `self.ReceiveTick`
  (params (DeltaSeconds :type "Float (single-precision)"))
  (if (`self.EndDelay`)
    (if (`self.TransformUp`)
      (`self.K2_AddActorLocalTransform` (`KismetMathLibrary.Conv_VectorToTransform` (* (`.Z` (`KismetMathLibrary.GetAxes` (* (`KismetMathLibrary.MakeRotator` 0.0 0.0 0.2) DeltaSeconds))) (0.0 0.0 0.3))) true)
      (`KismetSystemLibrary.Delay` 1.0)
      (set `self.TransformUp` false)
      (else
        (`self.K2_AddActorLocalTransform` (`KismetMathLibrary.Conv_VectorToTransform` (* (`.Z` (`KismetMathLibrary.GetAxes` (* (`KismetMathLibrary.MakeRotator` 0.0 0.0 0.2) DeltaSeconds))) (0.0 0.0 -0.3))) true)
        (`KismetSystemLibrary.Delay` 1.0)
        (set `self.TransformUp` true)))
    (else
      (`KismetSystemLibrary.Delay` (`KismetMathLibrary.RandomFloatInRange` 0.0 0.3))
      (set `self.EndDelay` true))))

(fn `UserConstructionScript`)