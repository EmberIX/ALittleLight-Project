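; Ghost enemy AI that patrols, haunts a lantern-bearing player and kills the player on capsule overlap.
; It loops AIMoveTo through up to four waypoint component locations cached at BeginPlay, while Tick alternates two timelines to pulse its point light.
; When a player with IsLantern set and LightChanged unset enters its sight range, it turns the light red, speeds up and chases, with no return to patrol.
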(event `SetWayPoint`
  (bind _waypoint_array (`self.Waypoint Array`))
  (bind _way_limit (`self.Way Limit`))
  (if (>= _way_limit 1)
    (`KismetArrayLibrary.Array_Add` _waypoint_array (`SceneComponent.K2_GetComponentLocation` (`self.Waypts01`)))
    (if (>= _way_limit 2)
      (`KismetArrayLibrary.Array_Add` _waypoint_array (`SceneComponent.K2_GetComponentLocation` (`self.Waypts02`)))
      (if (>= _way_limit 3)
        (`KismetArrayLibrary.Array_Add` _waypoint_array (`SceneComponent.K2_GetComponentLocation` (`self.Waypts03`)))
        (if (>= _way_limit 4)
          (`KismetArrayLibrary.Array_Add` _waypoint_array (`SceneComponent.K2_GetComponentLocation` (`self.Waypts04`))))))))

(event `self.ReceiveBeginPlay`
  (`self.SetWayPoint`)
  (`self.FollowWayPoint`)
  (`ParticleSystemComponent.EndTrails` (`self.GhostParticle`)))

(event `FollowWayPoint`
  (if (`self.WalkWayPoint`)
    (`|AIMoveTo` self (`|GetArrayItem` (`self.Waypoint Array`) (`self.WaypointNum`)) null 0.3
      (:`OnSuccess`
        (`KismetSystemLibrary.Delay` (`self.WaitTime`))
        (bind _output_get (set `self.WaypointNum` (+ (`self.WaypointNum`) 1)))
        (if (not (`KismetArrayLibrary.Array_IsValidIndex` (`self.Waypoint Array`) _output_get))
          (set `self.WaypointNum` 0 :!label _label)))
      (:`OnFail`
        (goto _label)))
    (`self.FollowWayPoint`)))

(event `self.ReceiveTick`
  (params (DeltaSeconds :type "Float (single-precision)"))
  (bind _pointlight (`self.PointLight`))
  (if (not (`self.HauntState`))
    (`/Engine/EditorBlueprintResources/StandardMacros.DoOnce` false :!label _label_2
      (:`Completed`
        (if (`self.LightUp`)
          (bind (_direction _intensity) (`Timeline|Timeline_0` :!via `ReverseFromEnd`)
            (:`Update`
              (`LightComponent.SetIntensity` _pointlight _intensity))
            (:`Finished`
              (set `self.LightUp` false)
              (goto _label_2 :!via `Reset`)))
          (else
            (bind (_direction_2 _intensity_2) (`Timeline|LightIntensity` :!via `PlayFromStart`)
              (:`Update`
                (`LightComponent.SetIntensity` _pointlight _intensity_2))
              (:`Finished`
                (set `self.LightUp` true)
                (goto _label_2 :!via `Reset`)))))))))

(event `self.SightRangee.OnComponentBeginOverlap`
  (params (OverlappedComponent :type "PrimitiveComponent Object Reference") (OtherActor :type "Actor Object Reference") (OtherComp :type "PrimitiveComponent Object Reference") (OtherBodyIndex :type Integer) (bFromSweep :type Boolean) (SweepResult :type "HitResult Structure (by ref)"))
  (bind _pointlight (`self.PointLight`))
  (bind _asthird_person_character (cast `/Game/Blueprints/ThirdPersonCharacter` OtherActor))
  (if (`/Game/Blueprints/ThirdPersonCharacter.IsLantern` _asthird_person_character)
    (if (not (`/Game/Blueprints/ThirdPersonCharacter.LightChanged` _asthird_person_character))
      (`KismetSystemLibrary.PrintString` "Haunting")
      (set `self.HauntState` true)
      (`LightComponent.SetIntensity` _pointlight 50.0)
      (`LightComponent.SetLightColor` _pointlight (struct :`R` 1.0 :`G` 0.008304 :`A` 1.0) true)
      (set `CharacterMovementComponent.MaxWalkSpeed` 1200.0 (`self.CharacterMovement`))
      (`|AIMoveTo` (`Controller.K2_GetPawn` (`self.GetController`)) (0.0 0.0 0.0) _asthird_person_character 0.1
        (:`then`
          (set `self.WalkWayPoint` false))))))

(event `self.CapsuleComponent.OnComponentBeginOverlap`
  (params (OverlappedComponent :type "PrimitiveComponent Object Reference") (OtherActor :type "Actor Object Reference") (OtherComp :type "PrimitiveComponent Object Reference") (OtherBodyIndex :type Integer) (bFromSweep :type Boolean) (SweepResult :type "HitResult Structure (by ref)"))
  (`|ExecutionSequence`
    (:`then_0`
      (bind _asthird_person_character (cast `/Game/Blueprints/ThirdPersonCharacter` OtherActor))
      (if (`PrimitiveComponent.IsOverlappingComponent` (`Character.CapsuleComponent` _asthird_person_character) OverlappedComponent)
        (`KismetSystemLibrary.PrintString` "Die")
        (`/Game/Blueprints/ThirdPersonCharacter.Die` _asthird_person_character)))))

(event `self.CapsuleComponent.OnComponentEndOverlap`
  (params (OverlappedComponent :type "PrimitiveComponent Object Reference") (OtherActor :type "Actor Object Reference") (OtherComp :type "PrimitiveComponent Object Reference") (OtherBodyIndex :type Integer))
  (`|ExecutionSequence`
    (:`then_0`
      (cast `/Game/Blueprints/ThirdPersonCharacter` OtherActor)
      (`KismetSystemLibrary.PrintString` "Bye"))))

(fn `UserConstructionScript`)