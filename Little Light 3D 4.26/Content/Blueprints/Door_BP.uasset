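; Locked door that takes the player's carried key and becomes a portal to another level.
; A proximity box shows a widget and enables Interact, which consumes the key, fades the door material, reveals the portal and toggles movement-blocking dialogue.
; Tick also consumes the key on Grab, without the fade.
; A second box, once unlocked, requires the lantern before showing a screen fade and opening the level after a delay.
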(event `self.ReceiveTick`
  (params (DeltaSeconds :type "Float (single-precision)"))
  (if (`self.isAtDoor`)
    (bind _asthird_person_character (cast `/Game/Blueprints/ThirdPersonCharacter` (`GameplayStatics.GetPlayerPawn` 0)))
    (if (`/Game/Blueprints/ThirdPersonCharacter.Grab` _asthird_person_character)
      (`|ExecutionSequence`
        (:`then_0`
          (bind _askey_bp (cast `/Game/Blueprints/Key_BP` (`/Game/Blueprints/ThirdPersonCharacter.CurrentAttach` _asthird_person_character))
            (:`then`
              (`|ExecutionSequence`
                (:`then_0`
                  (if (`/Game/Blueprints/ThirdPersonCharacter.isAttach` _asthird_person_character)
                    (`|ExecutionSequence`
                      (:`then_1`
                        (`self.K2_DestroyActor` _askey_bp)
                        (set `/Game/Blueprints/ThirdPersonCharacter.isAttach` false _asthird_person_character)
                        (set `self.isLock` false)
                        (set `self.Text` "I need my lantern.")))))))
            (:`CastFailed`
              (`KismetSystemLibrary.PrintString` "Cast Failed"))))))))

(event `/Game/Widget/UI/Interact_I.Interact`
  (if (`self.isAtDoor`)
    (`|ExecutionSequence`
      (:`then_0`
        (if (`self.isLock`)
          (bind _asthird_person_character (cast `/Game/Blueprints/ThirdPersonCharacter` (`GameplayStatics.GetPlayerPawn` 0)))
          (bind _askey_bp (cast `/Game/Blueprints/Key_BP` (`/Game/Blueprints/ThirdPersonCharacter.CurrentAttach` _asthird_person_character))
            (:`then`
              (`|ExecutionSequence`
                (:`then_0`
                  (if (`/Game/Blueprints/ThirdPersonCharacter.isAttach` _asthird_person_character)
                    (`self.K2_DestroyActor` _askey_bp)
                    (set `/Game/Blueprints/ThirdPersonCharacter.isAttach` false _asthird_person_character)
                    (set `self.isLock` false)
                    (set `/Game/Blueprints/ThirdPersonCharacter.isKey` false _asthird_person_character)
                    (set `self.Text` "I need my lantern.")))
                (:`then_1`
                  (bind (_direction _fading) (`Timeline|Fading` :!via `PlayFromStart`)
                    (:`Update`
                      (`MeshComponent.SetScalarParameterValueOnMaterials` (`self.Door`) "fadeOut" (`KismetMathLibrary.Lerp` 1.0 0.0 _fading))
                      (`SceneComponent.SetVisibility` (`self.Portal`) true true))))))
            (:`CastFailed`
              (`KismetSystemLibrary.PrintString` "Cast Failed")))))
      (:`then_1`
        (`/Engine/EditorBlueprintResources/StandardMacros.IsValid` (`self.DialogueWidget`)
          (:`Is Valid`
            (`Widget.RemoveFromParent` (`self.DialogueWidget`))
            (set `self.DialogueWidget` null)
            (bind _asthird_person_character_2 (cast `/Game/Blueprints/ThirdPersonCharacter` (`GameplayStatics.GetPlayerPawn` 0)))
            (set `/Game/Blueprints/ThirdPersonCharacter.CanWalk` true _asthird_person_character_2))
          (:`Is Not Valid`
            (bind _returnvalue (`|CreateWidget` "/Game/Widget/UI/DialogueBox.DialogueBox_C" (`GameplayStatics.GetPlayerController` 0)))
            (bind _output_get (set `self.DialogueWidget` _returnvalue))
            (`UserWidget.AddToViewport` _output_get 0)
            (set `/Game/Widget/UI/DialogueBox.DialogueText` (`self.Text`) (`self.DialogueWidget`))
            (bind _asthird_person_character_3 (cast `/Game/Blueprints/ThirdPersonCharacter` (`GameplayStatics.GetPlayerPawn` 0)))
            (set `/Game/Blueprints/ThirdPersonCharacter.CanWalk` false _asthird_person_character_3)))))))

(event `self.Box.OnComponentBeginOverlap`
  (params (OverlappedComponent :type "PrimitiveComponent Object Reference") (OtherActor :type "Actor Object Reference") (OtherComp :type "PrimitiveComponent Object Reference") (OtherBodyIndex :type Integer) (bFromSweep :type Boolean) (SweepResult :type "HitResult Structure (by ref)"))
  (bind _asthird_person_character (cast `/Game/Blueprints/ThirdPersonCharacter` OtherActor))
  (if (`PrimitiveComponent.IsOverlappingComponent` OverlappedComponent (`Character.CapsuleComponent` _asthird_person_character))
    (if (not (`self.isAtDoor`))
      (set `self.isAtDoor` true)
      (bind _asthird_person_character_2 (cast `/Game/Blueprints/ThirdPersonCharacter` (`GameplayStatics.GetPlayerPawn` 0)))
      (if (not (`/Game/Blueprints/ThirdPersonCharacter.isAtDoor` _asthird_person_character_2))
        (set `/Game/Blueprints/ThirdPersonCharacter.isAtDoor` true _asthird_person_character_2))
      (`SceneComponent.SetVisibility` (`self.Widget`) true false))))

(event `self.Box.OnComponentEndOverlap`
  (params (OverlappedComponent :type "PrimitiveComponent Object Reference") (OtherActor :type "Actor Object Reference") (OtherComp :type "PrimitiveComponent Object Reference") (OtherBodyIndex :type Integer))
  (bind _asthird_person_character (cast `/Game/Blueprints/ThirdPersonCharacter` OtherActor))
  (if (`PrimitiveComponent.IsOverlappingComponent` OverlappedComponent (`Character.CapsuleComponent` _asthird_person_character))
    _
    (elif (`self.isAtDoor`)
      (set `self.isAtDoor` false)
      (bind _asthird_person_character_2 (cast `/Game/Blueprints/ThirdPersonCharacter` (`GameplayStatics.GetPlayerPawn` 0)))
      (if (`/Game/Blueprints/ThirdPersonCharacter.isAtDoor` _asthird_person_character_2)
        (set `/Game/Blueprints/ThirdPersonCharacter.isAtDoor` false _asthird_person_character_2))
      (`SceneComponent.SetVisibility` (`self.Widget`) false false))))

(event `self.Box1.OnComponentBeginOverlap`
  (params (OverlappedComponent :type "PrimitiveComponent Object Reference") (OtherActor :type "Actor Object Reference") (OtherComp :type "PrimitiveComponent Object Reference") (OtherBodyIndex :type Integer) (bFromSweep :type Boolean) (SweepResult :type "HitResult Structure (by ref)"))
  ;[1 1 1] Door Change Scene
  (if (not (`self.isLock`))
    (bind _asthird_person_character (cast `/Game/Blueprints/ThirdPersonCharacter` OtherActor))
    (if (`PrimitiveComponent.IsOverlappingComponent` OverlappedComponent (`Character.CapsuleComponent` _asthird_person_character))
      (if (`/Game/Blueprints/ThirdPersonCharacter.IsLantern` _asthird_person_character)
        (`KismetSystemLibrary.PrintString` "ChangeScene")
        (bind _returnvalue (`|CreateWidget` "/Game/Widget/UI/Fading.Fading_C" (`GameplayStatics.GetPlayerController` 0)))
        (`UserWidget.AddToViewport` _returnvalue 0)
        (`self.NewLevel`)
        (else
          (`KismetSystemLibrary.PrintString` "Require Lantern"))))))

(event `NewLevel`
  (`KismetSystemLibrary.Delay` 1.0)
  (`KismetSystemLibrary.PrintString` "NewScene")
  (`GameplayStatics.OpenLevel` (`self.Level`)))

(fn `UserConstructionScript`)