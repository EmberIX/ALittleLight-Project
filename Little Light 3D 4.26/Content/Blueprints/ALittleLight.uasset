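; ALittleLight is an actor that travels along the spline of a referenced Track, presumably as a small moving light.
; On BeginPlay it starts the Move timeline, with play rate set from Duration and start time from StartOffset.
; Each update maps the timeline value to a distance along the spline and sets the actor's world location and rotation to match.
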(event `self.ReceiveBeginPlay`
  (bind _returnvalue (`KismetMathLibrary.Lerp` 0.0 (`SplineComponent.GetSplineLength` (`/Game/Blueprints/TrackRef.Spline` (`self.Track`))) (`self.Alpha`)))
  (`TimelineComponent.SetPlayRate` (`self.move`) (/ 1.0 (`self.Duration`)))
  (`TimelineComponent.SetNewTime` (`self.move`) (`self.StartOffset`))
  (bind (_direction _move) (`Timeline|move`)
    (:`Update`
      (set `self.Alpha` _move)
      (`self.K2_SetActorLocationAndRotation` (`SplineComponent.GetLocationAtDistanceAlongSpline` (`/Game/Blueprints/TrackRef.Spline` (`self.Track`)) _returnvalue "World") (`SplineComponent.GetRotationAtDistanceAlongSpline` (`/Game/Blueprints/TrackRef.Spline` (`self.Track`)) _returnvalue "World")))))

(event `self.ReceiveTick`
  (params (DeltaSeconds :type "Float (single-precision)")))

(fn `UserConstructionScript`)