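; End-level moving platform that, once activated, travels along the spline of a referenced Track actor.
; The Active event latches a flag so it runs only once, prints a debug message and plays the Moving timeline.
; The timeline's Travel value scales the spline length into a distance, setting the platform's world location and rotation, taking only roll and yaw from the spline.
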(event `self.ReceiveTick`
  (params (DeltaSeconds :type "Float (single-precision)")))

(event `self.ReceiveBeginPlay`)

(event `Active`
  (bind _spline (`/Game/Blueprints/TrackRef.Spline` (`self.Track`)))
  ;[1 1 1] Activated
  (if (not (`self.isActivated`))
    (`KismetSystemLibrary.PrintString` "Activate")
    (set `self.isActivated` true)
    (bind (_direction _travel) (`Timeline|Moving`)
      (:`Update`
        (bind _returnvalue (* _travel (`SplineComponent.GetSplineLength` (`/Game/Blueprints/TrackRef.Spline` (`self.Track`)))))
        (bind (_returnvalue_roll _returnvalue_pitch _returnvalue_yaw) (`KismetMathLibrary.BreakRotator` (`SplineComponent.GetRotationAtDistanceAlongSpline` _spline _returnvalue "World")))
        (`self.K2_SetActorLocationAndRotation` (`SplineComponent.GetLocationAtDistanceAlongSpline` _spline _returnvalue "World") (`KismetMathLibrary.MakeRotator` _returnvalue_roll 0.0 _returnvalue_yaw))))))

(fn `UserConstructionScript`)