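; BlueTree_BP is a tree actor that shows a widget when a ThirdPersonCharacter is nearby.
; Every Tick it turns UICircle on yaw only to face the player pawn.
; It also runs a zero-length sphere trace for pawns at its own location, showing Widget on a character hit and hiding it when nothing is hit.
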(event `self.ReceiveTick`
  (params (DeltaSeconds :type "Float (single-precision)"))
  (bind _returnvalue (`self.K2_GetActorLocation`))
  (bind _widget (`self.Widget`))
  (`|ExecutionSequence`
    (:`then_0`
      (`SceneComponent.K2_SetRelativeRotation` (`self.UICircle`) (`KismetMathLibrary.MakeRotator` 0.0 0.0 (.yaw (`KismetMathLibrary.FindLookAtRotation` (`SceneComponent.K2_GetComponentLocation` (`self.UICircle`)) (`self.K2_GetActorLocation` (`GameplayStatics.GetPlayerPawn` 0))))) false false))
    (:`then_1`
      (bind (_outhit _returnvalue_2) (`KismetSystemLibrary.SphereTraceSingleForObjects` _returnvalue _returnvalue 240.0 (`|MakeArray` "ObjectTypeQuery3" :!type "EObjectTypeQuery Enum") true))
      (if _returnvalue_2
        (cast `/Game/Blueprints/ThirdPersonCharacter` (`.HitActor` (`GameplayStatics.BreakHitResult` _outhit)))
        (`SceneComponent.SetVisibility` _widget true false)
        (else
          (`SceneComponent.SetVisibility` _widget false false))))))

(fn `UserConstructionScript`)