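; Ghost enemy that patrols up to four waypoints and chases the player on Bush overlap, killing them on capsule contact when outside light.
; Capsule overlaps track light sources (player lantern, lanterns, pillars, Koopa_BP2) in LightList, which drives IsInlight.
; Entering light cancels the haunt, resumes patrol and flashes a particle trail.
; A FadeOut timeline drives the mesh's fade parameter, reversing in light and playing forward when the last source leaves.
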(event `self.ReceiveBeginPlay`
  ;[1 1 1] BeginPlay
  (`ParticleSystemComponent.EndTrails` (`self.GhostParticle`))
  (`self.SetWayPoint`))

(event `self.ReceiveTick`
  (params (DeltaSeconds :type "Float (single-precision)")))

(event `FollowWayPoint`
  ;[1 1 1] FollowWayPoint
  (if (`self.WalkWayPoint`)
    (set `CharacterMovementComponent.MaxWalkSpeed` 230.0 (`self.CharacterMovement`))
    (if (not (`KismetArrayLibrary.Array_IsValidIndex` (`self.WaypointArray`) (`self.WaypointNum`)))
      (set `self.WaypointNum` 0))
    (`|AIMoveTo` self (`|GetArrayItem` (`self.WaypointArray`) (`self.WaypointNum`)) null 1.0
      (:`OnSuccess`
        (if (`KismetArrayLibrary.Array_Contains` (`self.WaitHere`) (`self.WaypointNum`))
          (`KismetSystemLibrary.Delay` (`self.WaitTime`)))
        (set `self.WaypointNum` (+ (`self.WaypointNum`) 1))
        (`self.FollowWayPoint`)))))

(event `self.Bush.OnComponentBeginOverlap`
  (params (OverlappedComponent :type "PrimitiveComponent Object Reference") (OtherActor :type "Actor Object Reference") (OtherComp :type "PrimitiveComponent Object Reference") (OtherBodyIndex :type Integer) (bFromSweep :type Boolean) (SweepResult :type "HitResult Structure (by ref)"))
  ;[1 1 1] Haunting
  (if (not (`self.isInlight`))
    (bind _asthird_person_character (cast `/Game/Blueprints/ThirdPersonCharacter` OtherActor :!label _label))
    (`KismetSystemLibrary.PrintString` "Haunting")
    (if (`self.ExitHaunting`)
      (`KismetSystemLibrary.Delay` 2.0)
      (set `self.ExitHaunting` false)
      (goto _label)
      (else
        (set `CharacterMovementComponent.MaxWalkSpeed` 550.0 (`self.CharacterMovement`))
        (`|AIMoveTo` (`Controller.K2_GetPawn` (`self.GetController`)) (0.0 0.0 0.0) _asthird_person_character 0.0
          (:`then`
            (set `self.WalkWayPoint` false)))))))

(event `SetWayPoint`
  (bind _waypointarray (`self.WaypointArray`))
  (bind _way_limit (`self.Way Limit`))
  ;[1 1 1] SetWayPoint
  (if (>= _way_limit 1)
    (`KismetArrayLibrary.Array_Add` _waypointarray (`SceneComponent.K2_GetComponentLocation` (`self.Waypts01`)))
    (if (>= _way_limit 2)
      (`KismetArrayLibrary.Array_Add` _waypointarray (`SceneComponent.K2_GetComponentLocation` (`self.Waypts02`)))
      (if (>= _way_limit 3)
        (`KismetArrayLibrary.Array_Add` _waypointarray (`SceneComponent.K2_GetComponentLocation` (`self.Waypts03`)))
        (if (>= _way_limit 4)
          (`KismetArrayLibrary.Array_Add` _waypointarray (`SceneComponent.K2_GetComponentLocation` (`self.Waypts04`)))))))
  (`self.FollowWayPoint`))

(event `Check Light`
  (bind _ghostparticle (`self.GhostParticle`))
  ;[1 1 1] Check Light/Player
  (`|ExecutionSequence` :!label _label_2
    (:`then_0`
      (bind _asthird_person_character (cast `/Game/Blueprints/ThirdPersonCharacter` (stale `self.CapsuleComponent.OnComponentBeginOverlap` OtherActor)))
      (if (`self.isInlight`)
        _
        (elif (`/Game/Blueprints/ThirdPersonCharacter.IsLantern` _asthird_person_character)
          (if (`/Game/Blueprints/ThirdPersonCharacter.LightChanged` _asthird_person_character)
            (if (`PrimitiveComponent.IsOverlappingComponent` (`Character.CapsuleComponent` _asthird_person_character) (stale `self.CapsuleComponent.OnComponentBeginOverlap` OverlappedComponent)) :!label _label_3
              (if (not (`self.isInlight`))
                (`KismetSystemLibrary.PrintString` "Die")
                (`/Game/Blueprints/ThirdPersonCharacter.Die` _asthird_person_character)))
            (else
              (`KismetArrayLibrary.Array_Add` (`self.LightList`) _asthird_person_character)
              (`KismetSystemLibrary.PrintString` "In light" :!label _label_4)
              (if (not (`self.isInlight`))
                (set `self.ExitHaunting` true)
                (`|ExecutionSequence` :!label _label_5
                  (:`then_0`
                    (if (> (`KismetArrayLibrary.Array_Length` (`self.LightList`)) 0)
                      (set `self.isInlight` true)
                      (`self.InLight`)))
                  (:`then_1`
                    (`ParticleSystemComponent.BeginTrails` _ghostparticle "None" "None" "ETrailWidthMode_FromCentre" 0.0)
                    (`KismetSystemLibrary.Delay` 0.5)
                    (`ParticleSystemComponent.EndTrails` _ghostparticle))))))
          (else
            (goto _label_3)))))
    (:`then_1`
      (bind _aslantern_bp (cast `/Game/Blueprints/Lantern_BP` (stale `self.CapsuleComponent.OnComponentBeginOverlap` OtherActor)))
      (if (`/Game/Blueprints/Lantern_BP.isLight` _aslantern_bp)
        (`KismetArrayLibrary.Array_Add` (`self.LightList`) _aslantern_bp)
        (goto _label_4)))
    (:`then_2`
      (bind _askoopa_bp2 (cast `/Game/Blueprints/Koopa_BP2` (stale `self.CapsuleComponent.OnComponentBeginOverlap` OtherActor)))
      (`KismetArrayLibrary.Array_Add` (`self.LightList`) _askoopa_bp2)
      (goto _label_5))
    (:`then_3`
      (bind _aspillar (cast `/Game/Blueprints/Pillar` (stale `self.CapsuleComponent.OnComponentBeginOverlap` OtherActor)))
      (`KismetArrayLibrary.Array_Add` (`self.LightList`) _aspillar)
      (goto _label_5))
    (:`then_4`
      (bind _asbroken_pillar (cast `/Game/Blueprints/BrokenPillar` (stale `self.CapsuleComponent.OnComponentBeginOverlap` OtherActor)))
      (if (`PrimitiveComponent.IsOverlappingComponent` (`/Game/Blueprints/BrokenPillar.Sphere1` _asbroken_pillar) (stale `self.CapsuleComponent.OnComponentBeginOverlap` OverlappedComponent))
        (if (`/Game/Blueprints/BrokenPillar.isLight` _asbroken_pillar)
          (`KismetArrayLibrary.Array_Add` (`self.LightList`) _asbroken_pillar)
          (goto _label_4))))))

(event `self.CapsuleComponent.OnComponentBeginOverlap`
  (params (OverlappedComponent :type "PrimitiveComponent Object Reference") (OtherActor :type "Actor Object Reference") (OtherComp :type "PrimitiveComponent Object Reference") (OtherBodyIndex :type Integer) (bFromSweep :type Boolean) (SweepResult :type "HitResult Structure (by ref)"))
  ;[1 1 1] Check Light/Player
  (goto _label_2))

(event `InLight`
  ;[1 1 1] InLight
  (if (`self.isInlight`)
    (bind (_direction _fade) (`Timeline|fadeOut` :!via `ReverseFromEnd` :!label _label_6)
      (:`Update`
        (`MeshComponent.SetScalarParameterValueOnMaterials` (`self.Mesh`) "fadeOut" (`KismetMathLibrary.Lerp` 1.0 0.0 _fade))
        (`|ExecutionSequence`
          (:`then_0`
            (set `self.ExitHaunting` false))
          (:`then_1`
            (set `self.WalkWayPoint` true)
            (`self.FollowWayPoint`)))))))

(event `OutLight`
  ;[1 1 1] OutLight
  (if (not (`self.isInlight`))
    (goto _label_6 :!via `PlayFromStart`)))

(event `self.CapsuleComponent.OnComponentEndOverlap`
  (params (OverlappedComponent :type "PrimitiveComponent Object Reference") (OtherActor :type "Actor Object Reference") (OtherComp :type "PrimitiveComponent Object Reference") (OtherBodyIndex :type Integer))
  ;[1 1 1] ExitLight
  (if (`self.isInlight`)
    (`|ExecutionSequence`
      (:`then_0`
        (bind _asthird_person_character (cast `/Game/Blueprints/ThirdPersonCharacter` OtherActor))
        (if (`/Game/Blueprints/ThirdPersonCharacter.IsLantern` _asthird_person_character)
          (if (`/Game/Blueprints/ThirdPersonCharacter.LightChanged` _asthird_person_character)
            _
            (elif (not (`PrimitiveComponent.IsOverlappingComponent` (`/Game/Blueprints/ThirdPersonCharacter.Sphere` _asthird_person_character) OverlappedComponent))
              (`KismetArrayLibrary.Array_RemoveItem` (`self.LightList`) _asthird_person_character)
              (if (not (> (`KismetArrayLibrary.Array_Length` (`self.LightList`)) 0)) :!label _label_7
                (set `self.isInlight` false)
                (`self.OutLight`))))))
      (:`then_1`
        (bind _aslantern_bp (cast `/Game/Blueprints/Lantern_BP` OtherActor))
        (if (`PrimitiveComponent.IsOverlappingComponent` (`/Game/Blueprints/Lantern_BP.LanternLightCol` _aslantern_bp) OverlappedComponent)
          _
          (elif (`/Game/Blueprints/Lantern_BP.isLight` _aslantern_bp)
            (`KismetArrayLibrary.Array_RemoveItem` (`self.LightList`) _aslantern_bp)
            (goto _label_7))))
      (:`then_2`
        (bind _askoopa_bp2 (cast `/Game/Blueprints/Koopa_BP2` OtherActor))
        (if (not (`PrimitiveComponent.IsOverlappingComponent` (`/Game/Blueprints/Koopa_BP2.SightRangee` _askoopa_bp2) OverlappedComponent))
          (`KismetArrayLibrary.Array_RemoveItem` (`self.LightList`) _askoopa_bp2)
          (goto _label_7)))
      (:`then_3`
        (bind _aspillar (cast `/Game/Blueprints/Pillar` OtherActor))
        (`KismetArrayLibrary.Array_RemoveItem` (`self.LightList`) _aspillar)
        (goto _label_7))
      (:`then_4`
        (bind _asbroken_pillar (cast `/Game/Blueprints/BrokenPillar` OtherActor))
        (if (`PrimitiveComponent.IsOverlappingComponent` (`/Game/Blueprints/BrokenPillar.Sphere1` _asbroken_pillar) OverlappedComponent)
          _
          (elif (`/Game/Blueprints/BrokenPillar.isLight` _asbroken_pillar)
            (`KismetArrayLibrary.Array_RemoveItem` (`self.LightList`) _asbroken_pillar)
            (goto _label_7)))))))

(fn `UserConstructionScript`)