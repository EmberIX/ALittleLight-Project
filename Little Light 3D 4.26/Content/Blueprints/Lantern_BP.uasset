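; Lantern actor that switches light, collision and appearance according to the player character's IsLantern and LightChanged flags, polled every Tick.
; IsLantern turns the light off and zeroes its collision sphere; otherwise, a sphere trace shows a widget when the player is near.
; LightChanged gives a dim orange light and red ball material, else a timeline grows a bright blue light and collision radius.
; The RootCover timeline fades root meshes through a material parameter.
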(event `self.ReceiveTick`
  (params (DeltaSeconds :type "Float (single-precision)"))
  (bind _returnvalue (`self.K2_GetActorLocation`))
  (bind _lanternlight (`self.LanternLight`))
  (bind _widget (`self.Widget`))
  (bind _lanternlightcol (`self.LanternLightCol`))
  (bind _asthird_person_character (cast `/Game/Blueprints/ThirdPersonCharacter` (`GameplayStatics.GetPlayerPawn` 0)))
  (`|ExecutionSequence`
    (:`then_0`
      (if (`/Game/Blueprints/ThirdPersonCharacter.IsLantern` _asthird_person_character)
        (`SphereComponent.SetSphereRadius` _lanternlightcol 0.0 true)
        (`ActorComponent.SetActive` _lanternlightcol false false)
        (`SceneComponent.SetVisibility` (`self.LanternLight`) false false)
        (set `self.isLight` false)
        (set `self.LightUpFinish` false)
        ;[1 1 1] set UI visible
        (`SceneComponent.SetVisibility` _widget false false :!label _label)
        (else
          (`|ExecutionSequence`
            (:`then_0`
              (bind (_outhit _returnvalue_2) (`KismetSystemLibrary.SphereTraceSingleForObjects` _returnvalue _returnvalue 70.0 (`|MakeArray` "ObjectTypeQuery3" :!type "EObjectTypeQuery Enum") true))
              (if _returnvalue_2
                (cast `/Game/Blueprints/ThirdPersonCharacter` (`.HitActor` (`GameplayStatics.BreakHitResult` _outhit)))
                (`SceneComponent.SetVisibility` _widget true false)
                (else
                  (goto _label))))
            (:`then_1`
              (if (`/Game/Blueprints/ThirdPersonCharacter.LightChanged` _asthird_person_character)
                (`ActorComponent.SetActive` (`self.LanternLightCol`) false false)
                (`SceneComponent.SetVisibility` _lanternlight true false)
                (`LightComponent.SetIntensity` _lanternlight 2.0)
                (`LocalLightComponent.SetAttenuationRadius` _lanternlight 70.0)
                (`LightComponent.SetLightColor` _lanternlight (struct :`R` 1.0 :`G` 0.341915 :`A` 1.0) true)
                (set `self.isLight` false)
                (else
                  (`self.SetLight`))))))))
    (:`then_1`
      (if (`/Game/Blueprints/ThirdPersonCharacter.LightChanged` _asthird_person_character)
        (`PrimitiveComponent.SetMaterial` (`self.Sphere`) 0 "/Game/Meterial/LightBallRed.LightBallRed")
        (bind (_direction _rootcover) (`Timeline|RootCover` :!via `Reverse` :!label _label_2)
          (:`Update`
            (`MeshComponent.SetScalarParameterValueOnMaterials` (`self.Root_Mesh`) "Appearance" (`KismetMathLibrary.Lerp` 1.0 0.0 _rootcover))))
        (else
          (`PrimitiveComponent.SetMaterial` (`self.Sphere`) 0 "/Game/Meterial/LightBall.LightBall")
          (goto _label_2))))))

(event `SetLight`
  (bind _lanternlightcol (`self.LanternLightCol`))
  (bind _lanternlight (`self.LanternLight`))
  (`ActorComponent.SetActive` _lanternlightcol true false)
  (if (not (`self.LightUpFinish`))
    (bind (_direction _lightup _lightcol) (`Timeline|Timeline_0` :!via `PlayFromStart`)
      (:`Update`
        (set `self.LightUpFinish` true)
        (`SphereComponent.SetSphereRadius` _lanternlightcol _lightcol true)
        (`SceneComponent.SetVisibility` _lanternlight true false)
        (`LightComponent.SetIntensity` _lanternlight _lightup)
        (`LocalLightComponent.SetAttenuationRadius` _lanternlight 500.0)
        (`LightComponent.SetLightColor` _lanternlight (struct :`R` 0.070701 :`G` 0.612894 :`B` 0.938686 :`A` 1.0) true)
        (set `self.isLight` true)))))

(fn `UserConstructionScript`)