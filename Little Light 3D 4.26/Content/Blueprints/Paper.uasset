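; Interactable paper actor that shows a readable document image on screen when the player interacts with it.
; BeginPlay creates a Picture widget, applies this actor's PaperUse texture to its image and caches the ThirdPersonCharacter.
; Interact toggles the widget: opening adds it to the viewport, plays a pickup sound and disables walking via CanWalk, and closing removes it and restores movement.
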(event `self.ReceiveBeginPlay`
  (bind _returnvalue (`|CreateWidget` "/Game/Widget/Picture/Picture.Picture_C" (`GameplayStatics.GetPlayerController` 0)))
  (set `self.paper` _returnvalue)
  (bind _asthird_person_character (cast `/Game/Blueprints/ThirdPersonCharacter` (`GameplayStatics.GetPlayerCharacter` 0)))
  (set `self.Player` _asthird_person_character)
  (`Image.SetBrushFromTexture` (`/Game/Widget/Picture/Picture.Paper` (`self.paper`)) (`self.Paper_Use`) false))

(event `/Game/Widget/UI/Interact_I.Interact`
  (bind _paper (`self.paper`))
  (if (`self.PaperOpen`)
    (`Widget.RemoveFromParent` _paper)
    (set `self.PaperOpen` false)
    (set `/Game/Blueprints/ThirdPersonCharacter.CanWalk` true (stale _output_get))
    (else
      (`UserWidget.AddToViewport` _paper 0)
      (`GameplayStatics.PlaySound2D` "/Game/Sound/Picking_up_paper_sound_effect.Picking_up_paper_sound_effect" 1.0 1.0 0.0 null null)
      (set `self.PaperOpen` true)
      (bind _output_get (set `self.Player` (`self.Player`)))
      (set `/Game/Blueprints/ThirdPersonCharacter.CanWalk` false _output_get))))

(event `self.ReceiveTick`
  (params (DeltaSeconds :type "Float (single-precision)")))

(fn `UserConstructionScript`)