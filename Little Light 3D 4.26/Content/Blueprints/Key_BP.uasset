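; Key actor that bobs in place with a ghost trail and shows a widget when the player character is near.
; While Transform is set, Tick nudges it up or down, flipping direction with a one-second Delay, and sphere-traces for the character to toggle the widget.
; When IsDetached is set, it returns to its BeginPlay transform, restarts the trail, resumes bobbing and clears the character's IsAttach flag.
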(event `self.ReceiveBeginPlay`
  (set `self.OriginalTransform` (`SceneComponent.K2_GetComponentToWorld` (`self.DefaultSceneRoot`)))
  (`ParticleSystemComponent.BeginTrails` (`self.GhostParticle`) "None" "None" "ETrailWidthMode_FromCentre" 0.0))

(event `self.ReceiveTick`
  (params (DeltaSeconds :type "Float (single-precision)"))
  (bind _returnvalue (`self.K2_GetActorLocation`))
  (bind _widget (`self.Widget`))
  (if (`self.isDetached`)
    (`ParticleSystemComponent.BeginTrails` (`self.GhostParticle`) "None" "None" "ETrailWidthMode_FromCentre" 0.0)
    (`self.ResetTransform`)
    (set `self.isDetached` false)
    (set `self.transform` true)
    (bind _asthird_person_character (cast `/Game/Blueprints/ThirdPersonCharacter` (`GameplayStatics.GetPlayerCharacter` 0)))
    (set `/Game/Blueprints/ThirdPersonCharacter.isAttach` false _asthird_person_character)
    (else
      (`|ExecutionSequence`
        (:`then_0`
          (if (`self.transform`)
            (`|ExecutionSequence`
              (:`then_0`
                (if (`self.TransformUp`)
                  (`self.K2_AddActorLocalTransform` (`KismetMathLibrary.Conv_VectorToTransform` (* (`.Z` (`KismetMathLibrary.GetAxes` (* (`KismetMathLibrary.MakeRotator` 0.0 0.0 0.2) DeltaSeconds))) (0.0 0.0 0.11))))
                  (`KismetSystemLibrary.Delay` 1.0)
                  (set `self.TransformUp` false)
                  (else
                    (`self.K2_AddActorLocalTransform` (`KismetMathLibrary.Conv_VectorToTransform` (* (`.Z` (`KismetMathLibrary.GetAxes` (* (`KismetMathLibrary.MakeRotator` 0.0 0.0 0.2) DeltaSeconds))) (0.0 0.0 -0.11))))
                    (`KismetSystemLibrary.Delay` 1.0)
                    (set `self.TransformUp` true))))
              (:`then_1`
                ;[1 1 1] set UI visible
                (bind (_outhit _returnvalue_2) (`KismetSystemLibrary.SphereTraceSingleForObjects` _returnvalue _returnvalue 70.0 (`|MakeArray` "ObjectTypeQuery3" :!type "EObjectTypeQuery Enum") true))
                (if _returnvalue_2
                  (cast `/Game/Blueprints/ThirdPersonCharacter` (`.HitActor` (`GameplayStatics.BreakHitResult` _outhit)))
                  (`SceneComponent.SetVisibility` _widget true false)
                  (else
                    (`SceneComponent.SetVisibility` _widget false false :!label _label)))))
            (else
              (goto _label))))))))

(fn `ResetTransform`
  (bind _defaultsceneroot (`self.DefaultSceneRoot`))
  (`SceneComponent.K2_SetWorldLocation` _defaultsceneroot (.location (`self.OriginalTransform`)) false false)
  (`SceneComponent.K2_SetWorldRotation` _defaultsceneroot (.rotation (`self.OriginalTransform`)) false false))

(fn `UserConstructionScript`)